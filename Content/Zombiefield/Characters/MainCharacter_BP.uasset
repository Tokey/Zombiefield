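; MainCharacter_BP is the main character Blueprint in Zombiefield, and its graph drives the on-screen HUD.
; On BeginPlay it creates an AmmoWidget_BP for the first player controller and adds it to the viewport.
; Every Tick it casts the stored widget and pushes current weapon ammo, score, health and rage mode text into it, polling rather than reacting to change events.
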(event `self.ReceiveBeginPlay`
  (bind _returnvalue (`|CreateWidget` "/Game/Zombiefield/HUD/AmmoWidget_BP.AmmoWidget_BP_C" (`GameplayStatics.GetPlayerController` 0)))
  (`UserWidget.AddToViewport` _returnvalue 0))

(event `self.ReceiveTick`
  (params (DeltaSeconds :type "Float (single-precision)"))
  (bind _asammo_widget_bp (cast `/Game/Zombiefield/HUD/AmmoWidget_BP` (stale `self.ReceiveBeginPlay` _returnvalue)))
  (`AmmoWidget.UpdateAmmoText` _asammo_widget_bp (`KismetStringLibrary.Conv_IntToString` (`.CurrentAmmoSize` (break `Ammo` (`Weapon.WeaponAmmo` (`self.CurrentWeapon`))))))
  (`AmmoWidget.UpdateScoreText` _asammo_widget_bp (`KismetStringLibrary.Conv_IntToString` (`self.Score`)))
  (`AmmoWidget.UpdateHealthText` _asammo_widget_bp (`KismetStringLibrary.Conv_IntToString` (`self.Health`)))
  (`AmmoWidget.UpdateRageModeText` _asammo_widget_bp (`self.RageModeText`)))

(fn `UserConstructionScript`)